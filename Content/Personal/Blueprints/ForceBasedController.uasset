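; A Character blueprint with mouse look, camera-relative movement and mouse-wheel zoom.
; The forward, right and vertical axis events share one path that rotates the input vector by control yaw and pitch before adding movement input.
; Each tick, the walkable floor angle scales with current speed relative to max speed, so faster movement allows steeper slopes.
; Wheel presses step the spring arm length in or out without limits.
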(event EventBeginPlay)

(event Collision|EventActorBeginOverlap
  (params (OtherActor :type Actor%20Object%20Reference)))

(event EventTick
  (params (DeltaSeconds :type Float%20%28single-precision%29))
  (bind _charactermovement (Variables|Character|GetCharacterMovement))
  (Pawn|Components|CharacterMovement|SetWalkableFloorAngle _charactermovement (Math|Float|Lerp 3e+01 7e+01 (/ (Math|Vector|VectorLength (Variables|/Script/Engine.MovementComponent|GetVelocity _charactermovement)) (Class|MovementComponent|GetMaxSpeed _charactermovement)))))

(event Input|AxisEvents|InputAxisMoveVertical
  (params (AxisValue :type Float%20%28single-precision%29))
  (bind _returnvalue (Pawn|GetControlRotation :!class /Script/Engine.Pawn))
  (if (> (Math|Vector|VectorLength (Math|Vector|RotateVectorAroundAxis (Math|Vector|RotateVectorAroundAxis (Math|Vector|MakeVector (stale Input|AxisEvents|InputAxisMoveForward/Backward AxisValue) (stale Input|AxisEvents|InputAxisMoveRight/Left AxisValue) AxisValue) (.yaw _returnvalue) (Math|Vector|VectorUp)) (.pitch _returnvalue) (* (Math|Vector|GetRightVector (Transformation|GetActorRotation)) "-1.000000,-1.000000,-1.000000"))) 0.0)
    (Pawn|Input|AddMovementInput (Math|Vector|RotateVectorAroundAxis (Math|Vector|RotateVectorAroundAxis (Math|Vector|MakeVector (stale Input|AxisEvents|InputAxisMoveForward/Backward AxisValue) (stale Input|AxisEvents|InputAxisMoveRight/Left AxisValue) AxisValue) (.yaw _returnvalue) (Math|Vector|VectorUp)) (.pitch _returnvalue) (* (Math|Vector|GetRightVector (Transformation|GetActorRotation)) "-1.000000,-1.000000,-1.000000")) 1.0 false)))

(event Input|AxisEvents|InputAxisMoveForward/Backward
  (params (AxisValue :type Float%20%28single-precision%29))
  (bind _returnvalue (Pawn|GetControlRotation :!class /Script/Engine.Pawn))
  (if (> (Math|Vector|VectorLength (Math|Vector|RotateVectorAroundAxis (Math|Vector|RotateVectorAroundAxis (Math|Vector|MakeVector AxisValue (stale Input|AxisEvents|InputAxisMoveRight/Left AxisValue) (stale Input|AxisEvents|InputAxisMoveVertical AxisValue)) (.yaw _returnvalue) (Math|Vector|VectorUp)) (.pitch _returnvalue) (* (Math|Vector|GetRightVector (Transformation|GetActorRotation)) "-1.000000,-1.000000,-1.000000"))) 0.0)
    (Pawn|Input|AddMovementInput (Math|Vector|RotateVectorAroundAxis (Math|Vector|RotateVectorAroundAxis (Math|Vector|MakeVector AxisValue (stale Input|AxisEvents|InputAxisMoveRight/Left AxisValue) (stale Input|AxisEvents|InputAxisMoveVertical AxisValue)) (.yaw _returnvalue) (Math|Vector|VectorUp)) (.pitch _returnvalue) (* (Math|Vector|GetRightVector (Transformation|GetActorRotation)) "-1.000000,-1.000000,-1.000000")) 1.0 false)))

(event Input|AxisEvents|InputAxisTurnRight/LeftMouse
  (params (AxisValue :type Float%20%28single-precision%29))
  ;[0.05098 0.05098 0.05098] Camera Input - Mouse
  (Pawn|Input|AddControllerYawInput AxisValue))

(event Input|AxisEvents|InputAxisLookUp/DownMouse
  (params (AxisValue :type Float%20%28single-precision%29))
  ;[0.05098 0.05098 0.05098] Camera Input - Mouse
  (Pawn|Input|AddControllerPitchInput AxisValue))

(event Input|AxisEvents|InputAxisMoveRight/Left
  (params (AxisValue :type Float%20%28single-precision%29))
  (bind _returnvalue (Pawn|GetControlRotation :!class /Script/Engine.Pawn))
  (if (> (Math|Vector|VectorLength (Math|Vector|RotateVectorAroundAxis (Math|Vector|RotateVectorAroundAxis (Math|Vector|MakeVector (stale Input|AxisEvents|InputAxisMoveForward/Backward AxisValue) AxisValue (stale Input|AxisEvents|InputAxisMoveVertical AxisValue)) (.yaw _returnvalue) (Math|Vector|VectorUp)) (.pitch _returnvalue) (* (Math|Vector|GetRightVector (Transformation|GetActorRotation)) "-1.000000,-1.000000,-1.000000"))) 0.0)
    (Pawn|Input|AddMovementInput (Math|Vector|RotateVectorAroundAxis (Math|Vector|RotateVectorAroundAxis (Math|Vector|MakeVector (stale Input|AxisEvents|InputAxisMoveForward/Backward AxisValue) AxisValue (stale Input|AxisEvents|InputAxisMoveVertical AxisValue)) (.yaw _returnvalue) (Math|Vector|VectorUp)) (.pitch _returnvalue) (* (Math|Vector|GetRightVector (Transformation|GetActorRotation)) "-1.000000,-1.000000,-1.000000")) 1.0 false)))

(event Input|MouseEvents|MouseWheelUp
  (params (Key :type Key%20Structure :default "None"))
  (:Pressed
    (bind _output_get (Variables|Default|SetZoom (- (Variables|Default|GetZoom) 5e+01)))
    (Variables|/Script/Engine.SpringArmComponent|SetTargetArmLength (Variables|Default|GetSpringArm) _output_get)))

(event Input|MouseEvents|MouseWheelDown
  (params (Key :type Key%20Structure :default "None"))
  (:Pressed
    (Variables|Default|SetZoom (+ (Variables|Default|GetZoom) 5e+01))
    (Variables|/Script/Engine.SpringArmComponent|SetTargetArmLength (Variables|Default|GetSpringArm) (stale Input|MouseEvents|MouseWheelUp _output_get))))

(fn ConstructionScript)