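; Player-controlled ball pawn that rolls via physics forces and carries a mouse-driven, zoomable camera.
; Mouse axes feed controller yaw and pitch input.
; Both movement axes share one path that sets MoveDirection scaled by Speed, rotates it by control yaw and applies it to the Sphere as acceleration.
; Mouse wheel steps the SpringArm length from its BeginPlay value, without clamping.
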(event EventBeginPlay
  (Variables|Default|SetZoom (Variables|/Script/Engine.SpringArmComponent|GetTargetArmLength (Variables|Default|GetSpringArm))))

(event Collision|EventActorBeginOverlap
  (params (OtherActor :type Actor%20Object%20Reference)))

(event EventTick
  (params (DeltaSeconds :type Float%20%28single-precision%29)))

(event Input|AxisEvents|InputAxisMoveForward/Backward
  (params (AxisValue :type Float%20%28single-precision%29))
  (bind _move_direction (Variables|Default|GetMove%20Direction))
  (bind _speed (Variables|Default|GetSpeed))
  (Class|KismetMathLibrary|VectorSet _move_direction (* AxisValue _speed) (* (stale Input|AxisEvents|InputAxisMoveRight/Left AxisValue) _speed) 0.0)
  (Physics|AddForce (Variables|Default|GetSphere) (Math|Vector|RotateVectorAroundAxis _move_direction (.yaw (Pawn|GetControlRotation :!class /Script/Engine.Pawn)) (Math|Vector|VectorUp)) "None" true))

(event Input|AxisEvents|InputAxisTurnRight/LeftMouse
  (params (AxisValue :type Float%20%28single-precision%29))
  ;[0.05098 0.05098 0.05098] Camera Input - Mouse
  (Pawn|Input|AddControllerYawInput AxisValue))

(event Input|AxisEvents|InputAxisLookUp/DownMouse
  (params (AxisValue :type Float%20%28single-precision%29))
  ;[0.05098 0.05098 0.05098] Camera Input - Mouse
  (Pawn|Input|AddControllerPitchInput AxisValue))

(event Input|AxisEvents|InputAxisMoveRight/Left
  (params (AxisValue :type Float%20%28single-precision%29))
  (bind _move_direction (Variables|Default|GetMove%20Direction))
  (bind _speed (Variables|Default|GetSpeed))
  (Class|KismetMathLibrary|VectorSet _move_direction (* (stale Input|AxisEvents|InputAxisMoveForward/Backward AxisValue) _speed) (* AxisValue _speed) 0.0)
  (Physics|AddForce (Variables|Default|GetSphere) (Math|Vector|RotateVectorAroundAxis _move_direction (.yaw (Pawn|GetControlRotation :!class /Script/Engine.Pawn)) (Math|Vector|VectorUp)) "None" true))

(event Input|MouseEvents|MouseWheelAxis
  (params (AxisValue :type Float%20%28single-precision%29)))

(event Input|MouseEvents|MouseWheelUp
  (params (Key :type Key%20Structure :default "None"))
  (:Pressed
    (bind _output_get (Variables|Default|SetZoom (- (Variables|Default|GetZoom) 5e+01)))
    (Variables|/Script/Engine.SpringArmComponent|SetTargetArmLength (Variables|Default|GetSpringArm) _output_get)))

(event Input|MouseEvents|MouseWheelDown
  (params (Key :type Key%20Structure :default "None"))
  (:Pressed
    (Variables|Default|SetZoom (+ (Variables|Default|GetZoom) 5e+01))
    (Variables|/Script/Engine.SpringArmComponent|SetTargetArmLength (Variables|Default|GetSpringArm) (stale Input|MouseEvents|MouseWheelUp _output_get))))

(fn ConstructionScript)