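; Door actor that opens once all of its linked Activators are on.
; On BeginPlay it binds to each activator's value change, raising or lowering a counter and opening when that count equals the array length.
; OpenDoor plays a timeline that lerps the Cube downward.
; An IsOpen RepNotify can also open the door, but the graph's only IsOpen setter is unconnected.
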(event Custom|Open%20Door
  (bind _open (Timeline|OpenAnim PlayFromStart)
    (:Update
      (Transformation|SetRelativeLocation (Variables|Default|GetCube) (Math|Vector|Lerp(Vector) "0, 0, 0" "0, 0,-300.000000" _open) false false))))

(event Custom|CheckConditions
  (params (ButtonIsOn :type Boolean))
  (bind _output_get (Variables|Default|SetAllTrue (+ (Variables|Default|GetAllTrue) (Math|Integer|SelectInt 1 -1 ButtonIsOn))))
  (Development|PrintString (Utilities|String|ToString(Integer) _output_get))
  (if (== _output_get (Utilities|Array|Length (Variables|Default|GetActivators)))
    (CallFunction|OpenDoor)))

(event EventBeginPlay
  (for _array_element (Variables|Default|GetActivators)
    (EventDispatchers|BindEventtoValueChanged _array_element (delegate Custom|CheckConditions))))

(event Collision|EventActorBeginOverlap
  (params (OtherActor :type Actor%20Object%20Reference)))

(event EventTick
  (params (DeltaSeconds :type Float%20%28single-precision%29)))

(fn ConstructionScript)

(fn OnRepIsOpen
  (if (Variables|Default|GetIsOpen)
    (CallFunction|OpenDoor)))