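; An interactable button actor that switches on when used and automatically switches back off after two seconds.
; InteractWith and ExecuteInteract ignore presses while it is on; otherwise they set IsOn, fire ValueChanged and start the reset timer.
; BeginPlay binds a handler to ValueChanged, and ChangeColorServer passes the state to ChangeColor, which tints the cube green for on and red for off.
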(event Custom|StartTimer
  (Utilities|FlowControl|Delay 2.0)
  (bind _output_get (Variables|Default|SetIsOn false))
  (Development|PrintString "Boop")
  (Default|CallValueChanged _output_get))

(event Custom|ChangeColor
  (params (ButtonIsOn :type Boolean))
  (Rendering|Material|SetVectorParameterValueonMaterials (Variables|Default|GetCube) "Color" (Math|Vector|SelectVector "0.000000,1.000000, 0" "1.000000, 0, 0" ButtonIsOn)))

(event Custom|ChangeColorServer
  (params (ButtonIsOn :type Boolean))
  (CallFunction|ChangeColor ButtonIsOn))

(event EventBeginPlay
  (EventDispatchers|BindEventtoValueChanged (EventDispatchers|CreateEvent :!event Custom|ChangeColor)))

(event Collision|EventActorBeginOverlap
  (params (OtherActor :type Actor%20Object%20Reference)))

(event EventTick
  (params (DeltaSeconds :type Float%20%28single-precision%29)))

(event EventExecuteInteract
  (if (not (Variables|Default|GetIsOn))
    (bind _output_get (Variables|Default|SetIsOn true))
    (Default|CallValueChanged _output_get)
    (CallFunction|StartTimer)))

(fn ConstructionScript)

(fn Interactwith
  (params (Interactor :type Astronaut%20Object%20Reference))
  (if (Variables|Default|GetIsOn)
    _
    (else
      (Development|PrintString "Beep")
      (bind _output_get (Variables|Default|SetIsOn true))
      (Default|CallValueChanged _output_get)
      (CallFunction|StartTimer)))
  (return (Variables|Default|GetIsOn)))

(fn Lookat
  (params (PlayerActor :type Astronaut%20Object%20Reference))
  (return "None"))