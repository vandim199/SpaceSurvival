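; Player-controlled spaceship pawn with mouse look and mouse-wheel camera zoom.
; Forward, strafe and vertical axes share one path that sets MoveDirection, rotates it by control yaw and passes it to AddMovementInput.
; The wheel steps the spring arm length without clamping.
; Speed-scaled impulse and movement alternatives are left unconnected, and the sphere overlap event is empty.
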(event OnComponentBeginOverlap(Sphere)
  (params (OverlappedComponent :type Primitive%20Component%20Object%20Reference) (OtherActor :type Actor%20Object%20Reference) (OtherComp :type Primitive%20Component%20Object%20Reference) (OtherBodyIndex :type Integer) (bFromSweep :type Boolean) (SweepResult :type Hit%20Result%20Structure%20%28by%20ref%29)))

(event EventBeginPlay)

(event Collision|EventActorBeginOverlap
  (params (OtherActor :type Actor%20Object%20Reference)))

(event EventTick
  (params (DeltaSeconds :type Float%20%28single-precision%29)))

(event Input|AxisEvents|InputAxisMoveVertical
  (params (AxisValue :type Float%20%28single-precision%29))
  (bind _move_direction (Variables|Default|GetMove%20Direction))
  (Class|KismetMathLibrary|VectorSet _move_direction (stale Input|AxisEvents|InputAxisMoveForward/Backward AxisValue) (stale Input|AxisEvents|InputAxisMoveRight/Left AxisValue) AxisValue)
  (Pawn|Input|AddMovementInput (Math|Vector|RotateVectorAroundAxis _move_direction (.yaw (Pawn|GetControlRotation :!class /Script/Engine.Pawn)) (Math|Vector|VectorUp)) 1.0 false))

(event Input|AxisEvents|InputAxisMoveForward/Backward
  (params (AxisValue :type Float%20%28single-precision%29))
  (bind _move_direction (Variables|Default|GetMove%20Direction))
  (Class|KismetMathLibrary|VectorSet _move_direction AxisValue (stale Input|AxisEvents|InputAxisMoveRight/Left AxisValue) (stale Input|AxisEvents|InputAxisMoveVertical AxisValue))
  (Pawn|Input|AddMovementInput (Math|Vector|RotateVectorAroundAxis _move_direction (.yaw (Pawn|GetControlRotation :!class /Script/Engine.Pawn)) (Math|Vector|VectorUp)) 1.0 false))

(event Input|AxisEvents|InputAxisTurnRight/LeftMouse
  (params (AxisValue :type Float%20%28single-precision%29))
  ;[0.05098 0.05098 0.05098] Camera Input - Mouse
  (Pawn|Input|AddControllerYawInput AxisValue))

(event Input|AxisEvents|InputAxisLookUp/DownMouse
  (params (AxisValue :type Float%20%28single-precision%29))
  ;[0.05098 0.05098 0.05098] Camera Input - Mouse
  (Pawn|Input|AddControllerPitchInput AxisValue))

(event Input|AxisEvents|InputAxisMoveRight/Left
  (params (AxisValue :type Float%20%28single-precision%29))
  (bind _move_direction (Variables|Default|GetMove%20Direction))
  (Class|KismetMathLibrary|VectorSet _move_direction (stale Input|AxisEvents|InputAxisMoveForward/Backward AxisValue) AxisValue (stale Input|AxisEvents|InputAxisMoveVertical AxisValue))
  (Pawn|Input|AddMovementInput (Math|Vector|RotateVectorAroundAxis _move_direction (.yaw (Pawn|GetControlRotation :!class /Script/Engine.Pawn)) (Math|Vector|VectorUp)) 1.0 false))

(event Input|MouseEvents|MouseWheelUp
  (params (Key :type Key%20Structure :default "None"))
  (:Pressed
    (bind _output_get (Variables|Default|SetZoom (- (Variables|Default|GetZoom) 5e+01)))
    (Variables|/Script/Engine.SpringArmComponent|SetTargetArmLength (Variables|Default|GetSpringArm) _output_get)))

(event Input|MouseEvents|MouseWheelDown
  (params (Key :type Key%20Structure :default "None"))
  (:Pressed
    (Variables|Default|SetZoom (+ (Variables|Default|GetZoom) 5e+01))
    (Variables|/Script/Engine.SpringArmComponent|SetTargetArmLength (Variables|Default|GetSpringArm) (stale Input|MouseEvents|MouseWheelUp _output_get))))

(fn ConstructionScript)