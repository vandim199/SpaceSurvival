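; Player-controlled spaceship pawn, going by its name, with mouse look and wheel zoom on a spring arm.
; Three movement axes share one path that rotates the input vector by control yaw into MoveDirection.
; Its RepNotify applies movement input scaled by Speed and prints the direction.
; Direct movement and MoveOnServer call chains remain in the graph unconnected.
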(event EventBeginPlay
  (Variables|Default|SetZoom (Variables|/Script/Engine.SpringArmComponent|GetTargetArmLength (Variables|Default|GetSpringArm))))

(event Collision|EventActorBeginOverlap
  (params (OtherActor :type Actor%20Object%20Reference)))

(event EventTick
  (params (DeltaSeconds :type Float%20%28single-precision%29)))

(event Input|AxisEvents|InputAxisMoveVertical
  (params (AxisValue :type Float%20%28single-precision%29))
  (bind _output_get (Variables|Default|SetMove%20Direction (Math|Vector|RotateVectorAroundAxis (Math|Vector|MakeVector (stale Input|AxisEvents|InputAxisMoveForward/Backward AxisValue) (stale Input|AxisEvents|InputAxisMoveRight/Left AxisValue) AxisValue) (.yaw (Pawn|GetControlRotation :!class /Script/Engine.Pawn)) (Math|Vector|VectorUp)))))

(event Input|AxisEvents|InputAxisMoveForward/Backward
  (params (AxisValue :type Float%20%28single-precision%29))
  (bind _output_get (Variables|Default|SetMove%20Direction (Math|Vector|RotateVectorAroundAxis (Math|Vector|MakeVector AxisValue (stale Input|AxisEvents|InputAxisMoveRight/Left AxisValue) (stale Input|AxisEvents|InputAxisMoveVertical AxisValue)) (.yaw (Pawn|GetControlRotation :!class /Script/Engine.Pawn)) (Math|Vector|VectorUp)))))

(event Input|AxisEvents|InputAxisTurnRight/LeftMouse
  (params (AxisValue :type Float%20%28single-precision%29))
  ;[0.05098 0.05098 0.05098] Camera Input - Mouse
  (Pawn|Input|AddControllerYawInput AxisValue))

(event Input|AxisEvents|InputAxisLookUp/DownMouse
  (params (AxisValue :type Float%20%28single-precision%29))
  ;[0.05098 0.05098 0.05098] Camera Input - Mouse
  (Pawn|Input|AddControllerPitchInput AxisValue))

(event Input|AxisEvents|InputAxisMoveRight/Left
  (params (AxisValue :type Float%20%28single-precision%29))
  (bind _output_get (Variables|Default|SetMove%20Direction (Math|Vector|RotateVectorAroundAxis (Math|Vector|MakeVector (stale Input|AxisEvents|InputAxisMoveForward/Backward AxisValue) AxisValue (stale Input|AxisEvents|InputAxisMoveVertical AxisValue)) (.yaw (Pawn|GetControlRotation :!class /Script/Engine.Pawn)) (Math|Vector|VectorUp)))))

(event Input|MouseEvents|MouseWheelAxis
  (params (AxisValue :type Float%20%28single-precision%29)))

(event Input|MouseEvents|MouseWheelUp
  (params (Key :type Key%20Structure))
  (:Pressed
    (bind _output_get (Variables|Default|SetZoom (- (Variables|Default|GetZoom) 5e+01)))
    (Variables|/Script/Engine.SpringArmComponent|SetTargetArmLength (Variables|Default|GetSpringArm) _output_get)))

(event Input|MouseEvents|MouseWheelDown
  (params (Key :type Key%20Structure))
  (:Pressed
    (Variables|Default|SetZoom (+ (Variables|Default|GetZoom) 5e+01))
    (Variables|/Script/Engine.SpringArmComponent|SetTargetArmLength (Variables|Default|GetSpringArm) (stale Input|MouseEvents|MouseWheelUp _output_get))))

(fn ConstructionScript)

(fn OnRepMoveDirection
  (bind _move_direction (Variables|Default|GetMove%20Direction))
  (Pawn|Input|AddMovementInput _move_direction (Variables|Default|GetSpeed) false)
  (Development|PrintString (Utilities|String|ToString(Vector) _move_direction)))