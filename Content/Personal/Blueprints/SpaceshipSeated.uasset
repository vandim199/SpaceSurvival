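; SpaceshipSeated is a possessable spaceship pawn that a player takes over by interacting with it.
; InteractWith runs on authority, calling PossessPawn on the interactor's DefaultPlayerController and returning its success.
; Mouse axes drive controller yaw and pitch, while forward, right and vertical axes share one movement path.
; That path rotates an axis-built vector by control yaw and pitch, then applies nonzero results as movement input.
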(event EventBeginPlay)

(event Collision|EventActorBeginOverlap
  (params (OtherActor :type Actor%20Object%20Reference)))

(event EventTick
  (params (DeltaSeconds :type Float%20%28single-precision%29)))

(event Input|AxisEvents|InputAxisMoveVertical
  (params (AxisValue :type Float%20%28single-precision%29))
  (bind _returnvalue (Pawn|GetControlRotation :!class /Script/Engine.Pawn))
  (if (> (Math|Vector|VectorLength (Math|Vector|RotateVectorAroundAxis (Math|Vector|RotateVectorAroundAxis (Math|Vector|MakeVector (stale Input|AxisEvents|InputAxisMoveForward/Backward AxisValue) (stale Input|AxisEvents|InputAxisMoveRight/Left AxisValue) AxisValue) (.yaw _returnvalue) (Math|Vector|VectorUp)) (.pitch _returnvalue) (* (Math|Vector|GetRightVector (Transformation|GetActorRotation)) "-1.000000,-1.000000,-1.000000"))) 0.0)
    (Pawn|Input|AddMovementInput (Math|Vector|RotateVectorAroundAxis (Math|Vector|RotateVectorAroundAxis (Math|Vector|MakeVector (stale Input|AxisEvents|InputAxisMoveForward/Backward AxisValue) (stale Input|AxisEvents|InputAxisMoveRight/Left AxisValue) AxisValue) (.yaw _returnvalue) (Math|Vector|VectorUp)) (.pitch _returnvalue) (* (Math|Vector|GetRightVector (Transformation|GetActorRotation)) "-1.000000,-1.000000,-1.000000")) 1.0 false)))

(event Input|AxisEvents|InputAxisMoveForward/Backward
  (params (AxisValue :type Float%20%28single-precision%29))
  (bind _returnvalue (Pawn|GetControlRotation :!class /Script/Engine.Pawn))
  (if (> (Math|Vector|VectorLength (Math|Vector|RotateVectorAroundAxis (Math|Vector|RotateVectorAroundAxis (Math|Vector|MakeVector AxisValue (stale Input|AxisEvents|InputAxisMoveRight/Left AxisValue) (stale Input|AxisEvents|InputAxisMoveVertical AxisValue)) (.yaw _returnvalue) (Math|Vector|VectorUp)) (.pitch _returnvalue) (* (Math|Vector|GetRightVector (Transformation|GetActorRotation)) "-1.000000,-1.000000,-1.000000"))) 0.0)
    (Pawn|Input|AddMovementInput (Math|Vector|RotateVectorAroundAxis (Math|Vector|RotateVectorAroundAxis (Math|Vector|MakeVector AxisValue (stale Input|AxisEvents|InputAxisMoveRight/Left AxisValue) (stale Input|AxisEvents|InputAxisMoveVertical AxisValue)) (.yaw _returnvalue) (Math|Vector|VectorUp)) (.pitch _returnvalue) (* (Math|Vector|GetRightVector (Transformation|GetActorRotation)) "-1.000000,-1.000000,-1.000000")) 1.0 false)))

(event Input|AxisEvents|InputAxisTurnRight/LeftMouse
  (params (AxisValue :type Float%20%28single-precision%29))
  (Pawn|Input|AddControllerYawInput AxisValue))

(event Input|AxisEvents|InputAxisLookUp/DownMouse
  (params (AxisValue :type Float%20%28single-precision%29))
  (Pawn|Input|AddControllerPitchInput AxisValue))

(event Input|AxisEvents|InputAxisMoveRight/Left
  (params (AxisValue :type Float%20%28single-precision%29))
  (bind _returnvalue (Pawn|GetControlRotation :!class /Script/Engine.Pawn))
  (if (> (Math|Vector|VectorLength (Math|Vector|RotateVectorAroundAxis (Math|Vector|RotateVectorAroundAxis (Math|Vector|MakeVector (stale Input|AxisEvents|InputAxisMoveForward/Backward AxisValue) AxisValue (stale Input|AxisEvents|InputAxisMoveVertical AxisValue)) (.yaw _returnvalue) (Math|Vector|VectorUp)) (.pitch _returnvalue) (* (Math|Vector|GetRightVector (Transformation|GetActorRotation)) "-1.000000,-1.000000,-1.000000"))) 0.0)
    (Pawn|Input|AddMovementInput (Math|Vector|RotateVectorAroundAxis (Math|Vector|RotateVectorAroundAxis (Math|Vector|MakeVector (stale Input|AxisEvents|InputAxisMoveForward/Backward AxisValue) AxisValue (stale Input|AxisEvents|InputAxisMoveVertical AxisValue)) (.yaw _returnvalue) (Math|Vector|VectorUp)) (.pitch _returnvalue) (* (Math|Vector|GetRightVector (Transformation|GetActorRotation)) "-1.000000,-1.000000,-1.000000")) 1.0 false)))

(fn ConstructionScript)

(fn Interactwith
  (params (Interactor :type Astronaut%20Object%20Reference))
  (bind _returnvalue (Pawn|GetController Interactor))
  (bind (_asdefault_player_controller _bsuccess) (Utilities|Casting|CastToDefaultPlayerController _returnvalue))
  (Networking|SwitchHasAuthority
    (:Authority
      (Default|PossessPawn _asdefault_player_controller Interactor self)
      (return _bsuccess))))

(fn Lookat
  (params (PlayerActor :type Astronaut%20Object%20Reference))
  (return "None"))